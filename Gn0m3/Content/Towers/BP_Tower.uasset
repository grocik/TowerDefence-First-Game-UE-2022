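; Base tower-defense turret that deducts gold from the arena actor on BeginPlay and attacks BP_Ghoul enemies once placed.
; Each Tick it picks the nearest ghoul by sphere overlap, rotates Top toward it and fires when cooled down and aligned.
; Fire branches on subclass: Balista spawns its projectile and applies instant damage, Cannon only spawns a projectile.
; The line-of-sight check is disconnected and PickProjectileBasedOnClass is an empty stub.
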(event `self.ReceiveBeginPlay`
  (bind _returnvalue (`GameplayStatics.GetActorOfClass` "/Game/ArenaLevel/ArenaActor.ArenaActor_C"))
  (bind _output_get (set `self.gold` _returnvalue))
  (set `/Game/ArenaLevel/ArenaActor.Gold` (- (`/Game/ArenaLevel/ArenaActor.Gold` _output_get) 5) _output_get))

(event `self.ReceiveTick`
  (params (DeltaSeconds :type "Float (single-precision)"))
  (if (`self.is Placed`)
    (`self.Find Best Target`)
    (`self.Target`
      (:`then`
        (`self.Update Turret Rotation`)
        (`self.Update Fite`))
      (:`else`))))

(event `Fire`
  (bind _returnvalue (`GameplayStatics.GetObjectClass` self))
  (bind _returnvalue_2 (`SceneComponent.GetSocketTransform` (`self.Top`) "FireSocket" "RTS_World"))
  (set `self.Time Of Last Fire` (`KismetSystemLibrary.GetGameTimeInSeconds`))
  (if (== _returnvalue "/Game/Towers/BP_Balista.BP_Balista_C")
    (`|SpawnActorFromClass` "/Game/Towers/BP_Projectile_Balista.BP_Projectile_Balista_C" _returnvalue_2 "Undefined" "OverrideRootScale" null null)
    (`GameplayStatics.ApplyDamage` (`self.besttarget`) 3.0)
    (elif (== _returnvalue "/Game/Towers/BP_Cannon.BP_Cannon_C")
      (`|SpawnActorFromClass` "/Game/Towers/BP_FirstPersonProjectile.BP_FirstPersonProjectile_C" _returnvalue_2 "Undefined" "OverrideRootScale" null null))))

(fn `Find Best Target`
  (locals (`Best Distance (local)` :type "Float (double-precision)") (`Current Distance (local)` :type "Float (double-precision)") (`Best Target (local)` :type "Actor Object Reference") (`Current Target (local)` :type "Actor Object Reference"))
  (set `local.Best Distance (local)` (+ (`self.Range`) 1.0))
  (bind _outactors (`KismetSystemLibrary.SphereOverlapActors` (`self.K2_GetActorLocation`) (`self.Range`) (`|MakeArray` "ObjectTypeQuery3" :!type "EObjectTypeQuery Enum") "/Game/UndeadPack/Ghoul/Blueprint/BP_Ghoul.BP_Ghoul_C"))
  (for _array_element _outactors
    (bind _output_get (set `local.Current Target (local)` _array_element))
    (bind _output_get_2 (set `local.Current Distance (local)` (`self.GetDistanceTo` _output_get self)))
    (if (or (< _output_get_2 (`local.Best Distance (local)`)) (not (`KismetSystemLibrary.IsValid` (`local.Best Target (local)`))))
      (if true
        (bind _output_get_3 (set `local.Best Target (local)` (`local.Current Target (local)`)))
        (set `local.Best Distance (local)` (`local.Current Distance (local)`))
        (set `self.besttarget` _output_get_3))))
  (set `self.Target` (`local.Best Target (local)`)))

(fn `Has Line Of Sight`
  (params (From :type "Vector Structure") (To :type "Vector Structure") (ActorsToIgnore :type "Array of Actor Object Reference (by ref)"))
  (returns (Result :type Boolean))
  (bind (_outhit _returnvalue) (`KismetSystemLibrary.LineTraceSingle` From To "TraceTypeQuery1" false ActorsToIgnore "None" false))
  (return (not _returnvalue)))

(fn `Pick Projectile Based On Class`
  (returns (NewParam :type "/Engine/Tutorial/BlueprintTutorials/ClassBlueprintsEditorOverview Class Reference"))
  (bind _returnvalue (`GameplayStatics.GetObjectClass` self))
  (if (== _returnvalue "/Game/Towers/BP_Balista.BP_Balista_C")
    (return null)
    (elif (== _returnvalue "/Game/Towers/BP_Cannon.BP_Cannon_C")
      (return null))))

(fn `Update Fite`
  (if (> (- (`KismetSystemLibrary.GetGameTimeInSeconds`) (`self.Time Of Last Fire`)) (`self.Rate Of Fire`))
    (if (> (`KismetMathLibrary.Dot_VectorVector` (`KismetMathLibrary.GetDirectionUnitVector` (`SceneComponent.K2_GetComponentLocation` (`self.Top`)) (`self.K2_GetActorLocation` (`self.Target`))) (`SceneComponent.GetForwardVector` (`self.Top`))) 0.99)
      (`self.Fire`))))

(fn `Update Turret Rotation`
  (`SceneComponent.K2_SetWorldRotation` (`self.Top`) (`KismetMathLibrary.RInterpTo_Constant` (`SceneComponent.K2_GetComponentRotation` (`self.Top`)) (`KismetMathLibrary.FindLookAtRotation` (`SceneComponent.K2_GetComponentLocation` (`self.Top`)) (`self.K2_GetActorLocation` (`self.Target`))) (`GameplayStatics.GetWorldDeltaSeconds`) (`self.Rotation Speed`)) false false))

(fn `UserConstructionScript`)